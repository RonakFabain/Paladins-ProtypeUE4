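; Hook projectile for Makoa that flies out briefly, then returns to where it spawned and destroys itself.
; BeginPlay stores the sphere's start location and, after a short delay, plays the Comeback timeline; a sphere hit also triggers it.
; Each timeline update zeroes projectile velocity and lerps the sphere from its current position toward the stored point, destroying the actor when finished.
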(event OnComponentHit(Sphere1)
  (params (HitComponent :type Primitive%20Component%20Object%20Reference) (OtherActor :type Actor%20Object%20Reference) (OtherComp :type Primitive%20Component%20Object%20Reference) (NormalImpulse :type Vector :default "0, 0, 0") (Hit :type Hit%20Result%20Structure%20%28by%20ref%29))
  (bind _newtrack_0 (Timeline|Comeback Play)
    (:Update
      (Variables|/Script/Engine.MovementComponent|SetVelocity (Variables|Default|GetProjectileMovement) "0, 0, 0")
      (Transformation|SetWorldLocation (Variables|Default|GetSphere1) (Math|Vector|Lerp(Vector) (Transformation|GetWorldLocation (Variables|Default|GetSphere1)) (stale EventBeginPlay _output_get) _newtrack_0) false false))
    (:Finished
      (Actor|DestroyActor))))

(event EventBeginPlay
  (bind _sphere1 (Variables|Default|GetSphere1))
  (bind _returnvalue (Transformation|GetWorldLocation _sphere1))
  (bind _output_get (Variables|Default|SetLocation _returnvalue))
  (Utilities|FlowControl|Delay 0.2)
  (bind _newtrack_0 (Timeline|Comeback Play)
    (:Update
      (Variables|/Script/Engine.MovementComponent|SetVelocity (Variables|Default|GetProjectileMovement) "0, 0, 0")
      (Transformation|SetWorldLocation (Variables|Default|GetSphere1) (Math|Vector|Lerp(Vector) _returnvalue _output_get _newtrack_0) false false))
    (:Finished
      (Actor|DestroyActor))))

(fn ConstructionScript)