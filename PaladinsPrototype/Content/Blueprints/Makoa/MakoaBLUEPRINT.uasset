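; Character Blueprint for Makoa, a playable hero with a dash roll on F and a hook on right mouse.
; Roll launches along the camera's forward vector, swapping to the third-person spring arm and hiding the weapon until ResetDash restores both and stops movement a second later.
; RMB spawns a Hook actor at the muzzle Scene, oriented by player controller 0.
; SpawnShield is an empty stub, and the Hook function only prints a debug string.
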(event EventBeginPlay
  (Variables|/Script/PaladinsPrototype.WeaponComponent|SetFP_MuzzleLocation (Variables|Default|GetWeaponComponent) (Variables|Default|GetScene)))

(event EventFRequestFunction
  (CallFunction|Roll)
  (Utilities|FlowControl|Delay 1.0)
  (CallFunction|ResetDash))

(event EventRMBRequestFunction
  (Game|SpawnActorfromClass "/Game/Blueprints/Makoa/Hook.Hook_C" (Math|Transform|MakeTransform (Transformation|GetWorldLocation (Variables|Default|GetScene)) (Math|Conversions|RotationFromXVector (* (Math|Vector|GetForwardVector (Variables|/Script/Engine.Actor|GetRootComponent (Game|GetPlayerController 0))) 2.0)) "1,1,1") "Undefined" 0 0))

(fn ConstructionScript)

(fn SpawnShield)

(fn Roll
  (bind _cameracomponent (Variables|Default|GetCameraComponent))
  (if (Variables|Default|GetbCanUseDash)
    (Components|Activation|Activate (Variables|Default|GetTPSSpringArm) false)
    (Components|Activation|Deactivate _cameracomponent)
    (Development|SetHiddeninGame (Variables|Default|GetWeaponMeshComponent) true false)
    (Character|LaunchCharacter (* (Math|Vector|GetForwardVector _cameracomponent) 2e+02) false false)
    (Variables|Default|SetbCanUseDash false)))

(fn Hook
  (Development|PrintString "rmb"))

(fn ResetDash
  (Variables|Default|SetbCanUseDash true)
  (Components|Activation|Deactivate (Variables|Default|GetTPSSpringArm))
  (Components|Activation|Activate (Variables|Default|GetCameraComponent) false)
  (Development|SetHiddeninGame (Variables|Default|GetWeaponMeshComponent) false false)
  (Components|Movement|StopMovementImmediately (Variables|Character|GetCharacterMovement)))